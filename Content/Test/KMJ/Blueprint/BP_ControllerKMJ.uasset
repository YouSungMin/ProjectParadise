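; BP_ControllerKMJ is a test controller that spawns familiars from number-key presses.
; On BeginPlay it finds the FamiliarSpawner actor in the level and caches it as AllySpawner.
; Keys 1 to 5 call SpawnFamiliarByID on that spawner with hardcoded IDs.
; Only key 1 names a familiar, BardFollower, while the other keys pass the placeholder ID "None".
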(event EventBeginPlay
  (bind _returnvalue (Actor|GetActorOfClass "/Script/Paradise.FamiliarSpawner"))
  (Variables|Default|SetAllySpawner _returnvalue))

(event Input|KeyboardEvents|1
  (params (Key :type Key%20Structure :default "None"))
  (:Pressed
    (Class|FamiliarSpawner|SpawnFamiliarbyID (Variables|Default|GetAllySpawner) "BardFollower")))

(event Input|KeyboardEvents|2
  (params (Key :type Key%20Structure :default "None"))
  (:Pressed
    (Class|FamiliarSpawner|SpawnFamiliarbyID (Variables|Default|GetAllySpawner) "None")))

(event Input|KeyboardEvents|3
  (params (Key :type Key%20Structure :default "None"))
  (:Pressed
    (Class|FamiliarSpawner|SpawnFamiliarbyID (Variables|Default|GetAllySpawner) "None")))

(event Input|KeyboardEvents|4
  (params (Key :type Key%20Structure :default "None"))
  (:Pressed
    (Class|FamiliarSpawner|SpawnFamiliarbyID (Variables|Default|GetAllySpawner) "None")))

(event Input|KeyboardEvents|5
  (params (Key :type Key%20Structure :default "None"))
  (:Pressed
    (Class|FamiliarSpawner|SpawnFamiliarbyID (Variables|Default|GetAllySpawner) "None")))

(fn ConstructionScript)